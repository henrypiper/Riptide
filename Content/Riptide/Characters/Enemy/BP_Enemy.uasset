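; BP_Enemy is an enemy that chases the player on sight and is destroyed when shot enough.
; PawnSensing sets a seeing flag, never cleared here, and starts an AI MoveTo toward the player character.
; On arrival it plays a rifle shoot montage behind a CanAttack gate and delay, with no damage dealt in this graph.
; Overlapping shooter bullets reduce Health through DamageEnemy, which destroys the actor at zero.
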(event `self.ReceiveActorBeginOverlap`
  (params (OtherActor :type "Actor Object Reference"))
  (cast `/Game/Riptide/Variant_Shooter/Blueprints/Pickups/Projectiles/BP_ShooterProjectile_Bullet` OtherActor)
  (`self.DamageEnemy` (`self.Bullet_damage`)))

(event `self.PawnSensing.OnSeePawn`
  (params (Pawn :type "Pawn Object Reference"))
  (set `self.isSeeingPlayer` true)
  (`self.Follow Player`))

(event `Follow Player`
  (set `self.canAttack` true)
  (if (`self.isSeeingPlayer`)
    (`|AIMoveTo` self (0.0 0.0 0.0) (`GameplayStatics.GetPlayerCharacter` 0) 50.0
      (:`OnSuccess`
        (if (`self.canAttack`)
          (set `self.canAttack` false)
          (bind _returnvalue (`self.PlayAnimMontage` "/Game/Riptide/Variant_Shooter/Anims/FP_Rifle_Shoot_Montage.FP_Rifle_Shoot_Montage"))
          (`KismetSystemLibrary.Delay` _returnvalue)
          (set `self.canAttack` true))))))

(fn `DamageEnemy`
  (params (DamageAmount :type "Float (double-precision)"))
  (bind _output_get (set `self.Health` (- (`self.Health`) DamageAmount)))
  (if (<= _output_get 0.0)
    (`self.K2_DestroyActor`)))

(fn `UserConstructionScript`)