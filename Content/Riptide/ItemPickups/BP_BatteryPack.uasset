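; BP_BatteryPack is a pickup that recharges the battery of BP_FirstPersonCharacter.
; Sphere overlap prints a debug string, then for that character adds a fixed amount to BatteryLife, clamped to a maximum, and destroys the pickup.
; Tick calls Spin, which yaws the actor and bobs it with a sine of game time, using per-frame offsets that are not scaled by delta time.
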(event `self.Sphere.OnComponentBeginOverlap`
  (params (OverlappedComponent :type "PrimitiveComponent Object Reference") (OtherActor :type "Actor Object Reference") (OtherComp :type "PrimitiveComponent Object Reference") (OtherBodyIndex :type Integer) (bFromSweep :type Boolean) (SweepResult :type "HitResult Structure (by ref)"))
  (`KismetSystemLibrary.PrintString` "Hello")
  (bind _asbp_first_person_character (cast `/Game/Riptide/FirstPerson/Blueprints/BP_FirstPersonCharacter` OtherActor))
  (set `/Game/Riptide/FirstPerson/Blueprints/BP_FirstPersonCharacter.BatteryLife` (`KismetMathLibrary.FClamp` (+ (`/Game/Riptide/FirstPerson/Blueprints/BP_FirstPersonCharacter.BatteryLife` _asbp_first_person_character) 5.0) 0.0 15.0) _asbp_first_person_character)
  (`self.K2_DestroyActor`))

(event `self.ReceiveTick`
  (params (DeltaSeconds :type "Float (single-precision)"))
  (`self.Spin` (1.0 1.0 1.0)))

(fn `Spin`
  (params (`New Transform Scale` :type "Vector Structure"))
  ; Add spin and bob
  ;; SPIN
  (`self.K2_AddActorLocalRotation` (struct :`Yaw` 1.0))
  ;; BOB
  (`self.K2_AddActorWorldOffset` (`KismetMathLibrary.MakeVector` 0.0 0.0 (* (`KismetMathLibrary.Sin` (* (`KismetSystemLibrary.GetGameTimeInSeconds`) 3.0)) 1.0))))

(fn `UserConstructionScript`)